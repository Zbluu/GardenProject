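; CultivablePlotBP is a plot Blueprint that shows dirt according to the plot's state and whether it is dry or wet.
; BeginPlay applies one dynamic material instance to all four dirt components, so a single parameter recolors them together, then calls UpdateAppearance.
; UpdateAppearance hides Dirt and its children in the Normal state and sets the shared Color parameter to the dry or wet color.
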(event EventBeginPlay
  ;[1 1 1] Create a material instance to be able to change the color of all the dirt components at once.
  (bind _returnvalue (Rendering|Material|CreateDynamicMaterialInstance "/Game/Meshes/Materials/DirtMaterial.DirtMaterial" "None" "None" :!class /Script/Engine.KismetMaterialLibrary))
  (bind _output_get (Variables|Default|SetDirtMaterialInstance _returnvalue))
  ;[1 1 1] Update all dirt materials with the dynamic one.
  (Rendering|Material|SetMaterial (Variables|Default|GetDirt) 0 _output_get)
  ;[1 1 1] Update appearance according to the variables.
  (CallFunction|UpdateAppearance))

(event EventTick
  (params (DeltaSeconds :type Float%20%28single-precision%29)))

(fn ConstructionScript)

(fn UpdateAppearance
  ;[1 1 1] Update the dirt visibility.
  (Rendering|SetVisibility (Variables|Default|GetDirt) (not (Utilities|Enum|Equal(Enum) (Class|CultivablePlot|GetState) "Normal")) true)
  ;[1 1 1] Update the dirt color according to if it's dry or wet.
  (Rendering|Material|SetVectorParameterValue (Variables|Default|GetDirtMaterialInstance) "Color" (Math|Color|SelectColor (Variables|Default|GetDryDirtColor) (Variables|Default|GetWetDirtColor) (Class|CultivablePlot|IsDry)) :!class /Script/Engine.MaterialInstanceDynamic))
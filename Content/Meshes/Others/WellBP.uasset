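; WellBP is a well actor that prompts the player to refill the watering can when in range.
; Overlap begin and end events on its SpherePlayerDetection component show and hide the refill text on the CharacterBP's HUD, but only while a WateringCanBP is equipped.
; Both events check player character 0 rather than the overlapping actor, and the refill itself is not handled here.
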(event OnComponentBeginOverlap(SpherePlayerDetection)
  (params (OverlappedComponent :type Primitive%20Component%20Object%20Reference) (OtherActor :type Actor%20Object%20Reference) (OtherComp :type Primitive%20Component%20Object%20Reference) (OtherBodyIndex :type Integer) (bFromSweep :type Boolean) (SweepResult :type Hit%20Result%20Structure%20%28by%20ref%29))
  (bind _ascharacter_bp (Utilities|Casting|CastToCharacterBP (Game|GetPlayerCharacter 0)))
  (Utilities|Casting|CastToWateringCanBP (Variables|/Game/Character/Blueprints/CharacterBP.CharacterBP_C|GetEquipedTool _ascharacter_bp))
  (Default|SetRefillWateringCanTextVisibility (Variables|/Game/Character/Blueprints/CharacterBP.CharacterBP_C|GetHUD _ascharacter_bp) true))

(event OnComponentEndOverlap(SpherePlayerDetection)
  (params (OverlappedComponent :type Primitive%20Component%20Object%20Reference) (OtherActor :type Actor%20Object%20Reference) (OtherComp :type Primitive%20Component%20Object%20Reference) (OtherBodyIndex :type Integer))
  (bind _ascharacter_bp (Utilities|Casting|CastToCharacterBP (Game|GetPlayerCharacter 0)))
  (Utilities|Casting|CastToWateringCanBP (Variables|/Game/Character/Blueprints/CharacterBP.CharacterBP_C|GetEquipedTool _ascharacter_bp))
  (Default|SetRefillWateringCanTextVisibility (Variables|/Game/Character/Blueprints/CharacterBP.CharacterBP_C|GetHUD _ascharacter_bp) false))

(event EventBeginPlay)

(event Collision|EventActorBeginOverlap
  (params (OtherActor :type Actor%20Object%20Reference)))

(event EventTick
  (params (DeltaSeconds :type Float%20%28single-precision%29)))

(fn ConstructionScript)